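; Chase boulder actor that rolls along a set direction behind the player, kills on overlap while CanKill is set, and carries a collectible key.
; Tick rubber-bands its speed around an ideal player distance, speeding up when far and slowing when close.
; If the player's Y falls below the boulder's, it returns to its start and resets obstacles and pots.
; Touching the key collision sets the character's HasKey and removes the key.
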(event `self.ReceiveBeginPlay`
  (set `self.speed` (`self.ideal speed`))
  (set `self.startpos` (`self.K2_GetActorLocation`)))

(event `self.ReceiveTick`
  (params (DeltaSeconds :type "Float (single-precision)"))
  (bind (_returnvalue_x _returnvalue_y) (`KismetMathLibrary.BreakVector` (`self.K2_GetActorLocation`)))
  (bind _idealdistance (`self.idealdistance`))
  (bind (_returnvalue_x_2 _returnvalue_y_2) (`KismetMathLibrary.BreakVector` (`self.K2_GetActorLocation` (`GameplayStatics.GetPlayerCharacter` 0))))
  (bind _returnvalue (`KismetMathLibrary.Vector_Distance` (`self.K2_GetActorLocation` (`GameplayStatics.GetPlayerCharacter` 0)) (`self.K2_GetActorLocation`)))
  (bind _returnvalue_2 (`KismetMathLibrary.Abs` (- _returnvalue _idealdistance)))
  (bind _returnvalue_3 (> _returnvalue_2 (`self.distance to reach max speed deviation`)))
  (bind _returnvalue_4 (* (/ _returnvalue_2 (`self.distance to reach max speed deviation`)) (`self.max speed deviation`)))
  (if (`self.Active`)
    (if (< _returnvalue_y_2 _returnvalue_y)
      (`self.K2_SetActorLocation` (`self.startpos`))
      (`self.RespawnBlocks`)
      (else
        (`self.K2_SetActorLocation` (+ (* DeltaSeconds (`self.direction`) (`self.speed`)) (`self.K2_GetActorLocation`)))
        (`SceneComponent.K2_SetWorldRotation` (`self.Sphere`) (`KismetMathLibrary.ComposeRotators` (`SceneComponent.K2_GetComponentRotation` (`self.Sphere`)) (`KismetMathLibrary.RotatorFromAxisAndAngle` (`KismetMathLibrary.Cross_VectorVector` (`self.direction`) (0.0 0.0 -1.0)) (/ (`self.speed`) 150.0))) false false)
        (if (> _returnvalue _idealdistance)
          (if _returnvalue_3
            (set `self.speed` (+ (`self.ideal speed`) (`self.max speed deviation`)))
            (else
              (set `self.speed` (+ _returnvalue_4 (`self.ideal speed`)))))
          (elif _returnvalue_3
            (set `self.speed` (+ (`self.ideal speed`) (* (`self.max speed deviation`) -1.0)))
            (else
              (set `self.speed` (+ (* _returnvalue_4 -1.0) (`self.ideal speed`))))))))))

(event `self.KeyCollision.OnComponentBeginOverlap`
  (params (OverlappedComponent :type "PrimitiveComponent Object Reference") (OtherActor :type "Actor Object Reference") (OtherComp :type "PrimitiveComponent Object Reference") (OtherBodyIndex :type Integer) (bFromSweep :type Boolean) (SweepResult :type "HitResult Structure (by ref)"))
  (bind _asbp_third_person_character (cast `/Game/Player/BP_ThirdPersonCharacter` OtherActor))
  (set `/Game/Player/BP_ThirdPersonCharacter.HasKey` true _asbp_third_person_character)
  (`ActorComponent.K2_DestroyComponent` (`self.KeyCollision`))
  (`ActorComponent.K2_DestroyComponent` (`self.Key`))
  (`AudioComponent.Play` (`self.CollectKey`) 0.0))

(event `self.Box.OnComponentBeginOverlap`
  (params (OverlappedComponent :type "PrimitiveComponent Object Reference") (OtherActor :type "Actor Object Reference") (OtherComp :type "PrimitiveComponent Object Reference") (OtherBodyIndex :type Integer) (bFromSweep :type Boolean) (SweepResult :type "HitResult Structure (by ref)"))
  (if (`self.CanKill`)
    (bind _asbp_third_person_character (cast `/Game/Player/BP_ThirdPersonCharacter` OtherActor))
    (`/Game/Player/Death/BPC_DeathComponent.Execute Death Sequence` (`self.GetComponentByClass` _asbp_third_person_character "/Game/Player/Death/BPC_DeathComponent.BPC_DeathComponent_C"))))

(event `GoDown`
  (if (not (`self.CanKill`))
    (set `self.direction` (0.0 0.0 0.0))
    (`SceneComponent.K2_AddWorldOffset` (`self.Sphere`) (0.0 0.0 -2.5) false true)))

(fn `RespawnBlocks`
  (bind _outactors (`GameplayStatics.GetAllActorsOfClass` "/Game/Assets/BoulderChase/AlphaEnding/BP_ChaseObstacle.BP_ChaseObstacle_C"))
  (for _array_element _outactors
    (`/Game/Assets/BoulderChase/AlphaEnding/BP_ChaseObstacle.Reset` _array_element))
  (bind _outactors_2 (`GameplayStatics.GetAllActorsOfClass` "/Game/Assets/PotsAndCoins/Pot.Pot_C"))
  (for _array_element_2 _outactors_2
    (`/Game/Assets/PotsAndCoins/Pot.Reset` _array_element_2)))

(fn `UserConstructionScript`)