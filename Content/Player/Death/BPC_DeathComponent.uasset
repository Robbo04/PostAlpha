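; BPC_DeathComponent is a player component that handles death by fading the screen and teleporting its owner to a respawn point.
; On BeginPlay it saves the owner's location as a fallback respawn point and creates a WBP_UIFade widget.
; ExecuteDeathSequence starts the fade and opens a Tick-driven timer, which teleports the owner after half a second to sync with the fade.
; UpdateRespawnLocation lets other logic move the respawn point.
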(event `self.ReceiveBeginPlay`
  ;[1 1 1] Safety script to make sure the player can always respawn
  (set `self.RespawnLocation` (`Actor.K2_GetActorLocation` (`self.GetOwner`)))
  (bind _returnvalue (`|CreateWidget` "/Game/Player/Death/WBP_UIFade.WBP_UIFade_C" (`PlayerState.GetPlayerController` (`GameplayStatics.GetPlayerState` 0))))
  (`UserWidget.AddToViewport` _returnvalue 0)
  (set `self.UI Fade Object Reference` _returnvalue))

(event `self.ReceiveTick`
  (params (DeltaSeconds :type "Float (single-precision)"))
  ;[1 1 1] Timer is used here so the teleportation can be timed with the UI fade
  (if (`self.RespawnTimerOpen`)
    (bind _output_get (set `self.RespawnTimer` (+ DeltaSeconds (`self.RespawnTimer`))))
    (if (>= _output_get 0.5)
      ;[1 1 1] If the Timer is at .5 seconds then teleport the player and close the respawn timer gate and also reset the respawn timer for next usage
      (`Actor.K2_SetActorLocation` (`self.GetOwner`) (`self.RespawnLocation`) false true)
      (set `self.RespawnTimer` 0.0)
      (set `self.RespawnTimerOpen` false))))

(fn `Execute Death Sequence`
  (`/Game/Player/Death/WBP_UIFade.Fade Out And In` (`self.UI Fade Object Reference`))
  (set `self.RespawnTimerOpen` true))

(fn `UpdateRespawnLocation`
  (params (RespawnLocation :type "Vector Structure"))
  (set `self.RespawnLocation` RespawnLocation))